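; Environment tile that triggers a level-up when any actor begins overlapping it.
; After running the parent overlap logic, it finds the BP_Treadmill in the level and calls LevelUp on it.
; It then resets OpacityCurveTime on the UWHUD widget of player 0's BP_HUD, which suggests it restarts an opacity animation.
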(event `self.ReceiveActorBeginOverlap`
  (params (OtherActor :type "Actor Object Reference"))
  (`parent.ReceiveActorBeginOverlap` OtherActor)
  (bind _returnvalue (`GameplayStatics.GetActorOfClass` "/Game/Environment/BP_Treadmill.BP_Treadmill_C"))
  (`/Game/Environment/BP_Treadmill.LevelUp` _returnvalue)
  (bind _asbp_hud (cast `/Game/Blueprints/BP_HUD` (`PlayerController.GetHUD` (`GameplayStatics.GetPlayerController` 0))))
  (set `/Game/UI/UW_HUD.Opacity Curve Time` 0.0 (`/Game/Blueprints/BP_HUD.UW_HUD` _asbp_hud)))

(fn `UserConstructionScript`
  (`parent.UserConstructionScript`))