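; BP_PlayerController is the player controller Blueprint that holds player health and triggers game over.
; HealthSetter stores the new Health and, at zero or below, pauses the game, removes the BP_HUD widget and shows a newly created UW_GameOver widget.
; BeginPlay and Tick are empty, and an unconnected CreateSaveGameObject node never runs.
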(fn `HealthSetter`
  (params (Health :type Integer))
  (bind _output_get (set `self.Health` Health))
  (if (<= _output_get 0)
    ;[1 1 1] Game Over
    (`GameplayStatics.SetGamePaused` true)
    (bind _asbp_hud (cast `/Game/UI/BP_HUD` (`self.GetHUD` (`GameplayStatics.GetPlayerController` 0))))
    (`Widget.RemoveFromParent` (`/Game/UI/BP_HUD.UW_HUD` _asbp_hud))
    (bind _returnvalue (`|CreateWidget` "/Game/UI/UW_GameOver.UW_GameOver_C"))
    (`UserWidget.AddToViewport` _returnvalue 0)))

(fn `UserConstructionScript`)